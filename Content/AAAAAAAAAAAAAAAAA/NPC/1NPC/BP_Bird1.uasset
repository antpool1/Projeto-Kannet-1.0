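; BP_Bird1 is a bird NPC character that can fly toward a given target location.
; The Fly event stores the target and switches CharacterMovement to Flying mode.
; While in that mode, Tick steers straight at the target with normalized movement input, with no arrival check or switch back to another mode.
; IsFlying reports whether the bird is in Flying mode.
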(event EventBeginPlay)

(event Collision|EventActorBeginOverlap
  (params (OtherActor :type Actor%20Object%20Reference)))

(event EventTick
  (params (DeltaSeconds :type Float%20%28single-precision%29))
  (switch Utilities|FlowControl|Switch|SwitchonEMovementMode (Variables|/Script/Engine.CharacterMovementComponent|GetMovementMode (Variables|Character|GetCharacterMovement))
    (:MOVE_Flying
      (|FlyingMoviment))))

(event EventFly
  (params (Target :type Vector :default "0, 0, 0"))
  (Variables|Default|SetFly%20Target%20Location Target)
  (Pawn|Components|CharacterMovement|SetMovementMode (Variables|Character|GetCharacterMovement) "MOVE_Flying" 0))

(fn ConstructionScript)

(fn IsFlying
  (return (Utilities|Enum|Equal(Enum) (Variables|/Script/Engine.CharacterMovementComponent|GetMovementMode (Variables|Character|GetCharacterMovement)) "MOVE_Flying")))