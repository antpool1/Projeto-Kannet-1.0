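; Enemy NPC that chases the player on sight, attacks in melee and can be assassinated from behind.
; Pawn sensing triggers AI MoveTo, then a montage and sphere-overlap damage, with movement halted during attacks; damage drains health until destruction.
; An overlap radius shows a camera-facing assassinate prompt to the player.
; StealthBackAssassin plays the victim montage, returns an alignment transform and triggers delayed ragdoll; behavior-tree blackboard code is unconnected.
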(event OnSeePawn(PawnSensing)
  (params (Pawn :type Pawn%20Object%20Reference))
  (Variables|Default|SetisSeenThePlayer? true)
  (CallFunction|FollowPlayer))

(event OnComponentBeginOverlap(AssassinationRadius)
  (params (OverlappedComponent :type Primitive%20Component%20Object%20Reference) (OtherActor :type Actor%20Object%20Reference) (OtherComp :type Primitive%20Component%20Object%20Reference) (OtherBodyIndex :type Integer) (bFromSweep :type Boolean) (SweepResult :type Hit%20Result%20Structure%20%28by%20ref%29))
  (Utilities|Casting|CastToBP_ThirdPersonCharacter OtherActor)
  (Rendering|SetVisibility (Variables|Default|GetWidget1Assassinate) true false))

(event OnComponentEndOverlap(AssassinationRadius)
  (params (OverlappedComponent :type Primitive%20Component%20Object%20Reference) (OtherActor :type Actor%20Object%20Reference) (OtherComp :type Primitive%20Component%20Object%20Reference) (OtherBodyIndex :type Integer))
  (Utilities|Casting|CastToBP_ThirdPersonCharacter OtherActor)
  (Rendering|SetVisibility (Variables|Default|GetWidget1Assassinate) false false))

(event Custom|Follow%20Player
  (Variables|Default|SetCanAttack? true)
  (if (Variables|Default|GetisSeenThePlayer?)
    (AI|AIMoveTo self "0, 0, 0" (Game|GetPlayerCharacter 0) 5.0 false
      (:OnSuccess
        (if (Variables|Default|GetCanAttack?)
          (Variables|Default|SetCanAttack? false)
          (bind _returnvalue (Animation|PlayAnimMontage "/Game/AAAAAAAAAAAAAAAAA/NPC/Enemy_NPC/2/Anime_Heraklios/P1_Heraklios.P1_Heraklios" 1.0 "None"))
          (bind _outactors (Collision|SphereOverlapActors (Transformation|GetWorldLocation (Variables|Default|GetArrow1)) 1e+02 (Variables|Default|GetObject%20Types) 0))
          (bind _array_element (Utilities|Array|ForEachLoopwithBreak _outactors)
            (:LoopBody
              (if (Actor|ActorHasTag _array_element "Player")
                (Game|Damage|ApplyDamage _array_element 2e+01 0 0)))
            (:Completed
              (Utilities|FlowControl|Delay _returnvalue)
              (Variables|Default|SetCanAttack? true))))))
    (else
      (Variables|Default|SetisSeenThePlayer? false))))

(event Custom|Ragdoll
  ;[1 1 1] BP Ragdoll
  (Utilities|FlowControl|Delay 6.05)
  (Physics|SetSimulatePhysics (Variables|Character|GetMesh) true))

(event EventTick
  (params (DeltaSeconds :type Float%20%28single-precision%29))
  (Utilities|FlowControl|Sequence
    (:then_0
      (if (not (Variables|Default|GetCanAttack?))
        (Components|Movement|StopMovementImmediately (Variables|Character|GetCharacterMovement))))
    (:then_1
      ;[1 1 1 1 100] Make The LifeWidget Look at Camera (Only if you have one camera
      (Transformation|SetWorldRotation (Variables|Default|GetWidget) (Math|Rotator|FindLookatRotation (Transformation|GetWorldLocation (Variables|/Script/Engine.PlayerCameraManager|GetTransformComponent (Game|GetPlayerCameraManager 3))) (Transformation|GetWorldLocation (Variables|Default|GetWidget))) false false))
    (:then_2
      (Transformation|SetWorldRotation (Variables|Default|GetWidget1Assassinate) (Math|Rotator|FindLookatRotation (Transformation|GetWorldLocation (Variables|Default|GetWidget1Assassinate)) (Transformation|GetWorldLocation (Variables|/Script/Engine.PlayerCameraManager|GetTransformComponent (Game|GetPlayerCameraManager 0)))) false false))))

(event Game|Damage|EventAnyDamage
  (params (Damage :type Float%20%28single-precision%29) (DamageType :type Damage%20Type%20Object%20Reference) (InstigatedBy :type Controller%20Object%20Reference) (DamageCauser :type Actor%20Object%20Reference))
  ;[1 1 1] BP Recive Damage
  (Variables|Default|SetHealth (- (Variables|Default|GetHealth) Damage))
  (Development|PrintString "Hello")
  (if (<= (Variables|Default|GetHealth) 0.0)
    (Actor|DestroyActor)))

(fn ConstructionScript)

(fn StealthBackAssassin
  (Animation|PlayAnimMontage "/Game/AAAAAAAAAAAAAAAAA/NPC/Enemy_NPC/2/Finalizacao/B1_Hell_Slammer_B_Montage.B1_Hell_Slammer_B_Montage" 1.0 "None")
  (Rendering|SetVisibility (Variables|Default|GetWidget1Assassinate) false false)
  (CallFunction|Ragdoll)
  (return (Transformation|GetWorldLocation (Variables|Default|GetRef%20Assassin)) (Transformation|GetActorRotation)))