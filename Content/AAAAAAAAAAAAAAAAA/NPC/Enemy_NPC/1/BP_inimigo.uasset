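; Enemy NPC character that the player can take down in stealth.
; A takedown box sets CanTakeDown on BP_ThirdPersonCharacter while the player overlaps it.
; The takedown event disables movement and collision, plays the victim montage, waits for its length, then destroys the actor.
; A helper function line-traces forward from the actor for surface attachment, though nothing in this file calls it.
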(event OnComponentBeginOverlap(TakedownBoxCollision)
  (params (OverlappedComponent :type Primitive%20Component%20Object%20Reference) (OtherActor :type Actor%20Object%20Reference) (OtherComp :type Primitive%20Component%20Object%20Reference) (OtherBodyIndex :type Integer) (bFromSweep :type Boolean) (SweepResult :type Hit%20Result%20Structure%20%28by%20ref%29))
  ;[1 1 1] This BP is if i can Atack or Not The Enemy in Stealth
  ;;[1 1 1] Cast The Player
  (bind _asbp_third_person_character (Utilities|Casting|CastToBP_ThirdPersonCharacter OtherActor))
  ;;[1 1 1] False or True
  (Variables|/Game/ThirdPerson/Blueprints/BP_ThirdPersonCharacter.BP_ThirdPersonCharacter_C|SetCanTakeDown? _asbp_third_person_character true))

(event OnComponentEndOverlap(TakedownBoxCollision)
  (params (OverlappedComponent :type Primitive%20Component%20Object%20Reference) (OtherActor :type Actor%20Object%20Reference) (OtherComp :type Primitive%20Component%20Object%20Reference) (OtherBodyIndex :type Integer))
  ;[1 1 1] This BP is if i can Atack or Not The Enemy in Stealth
  ;;[1 1 1] Cast The Player
  (bind _asbp_third_person_character (Utilities|Casting|CastToBP_ThirdPersonCharacter OtherActor))
  ;;[1 1 1] False or True
  (Variables|/Game/ThirdPerson/Blueprints/BP_ThirdPersonCharacter.BP_ThirdPersonCharacter_C|SetCanTakeDown? _asbp_third_person_character false))

(event Custom|Custom%20event%20Take%20down
  ;[1 1 1] Custom event To Chose Any Animation Montage in the Ceene
  (Pawn|Components|CharacterMovement|DisableMovement (Variables|Character|GetCharacterMovement))
  (Collision|SetActorEnableCollision false)
  (bind _returnvalue (Animation|PlayAnimMontage "/Game/AAAAAAAAAAAAAAAAA/NPC/Enemy_NPC/1/Animations/Vict_AM.Vict_AM" 1.0 "None"))
  (Utilities|FlowControl|Delay _returnvalue)
  (Actor|DestroyActor))

(fn ConstructionScript)

(fn AttatchtoSurfaceCalculation
  (params (Attatch%20Distance :type Float%20%28single-precision%29))
  (bind _returnvalue (Transformation|GetActorLocation))
  (bind (_outhit _returnvalue_2) (Collision|LineTraceByChannel _returnvalue (+ _returnvalue (* (Math|Vector|GetForwardVector (Transformation|GetActorRotation)) Attatch%20Distance)) "TraceTypeQuery1" false 0 "None"))
  (return _outhit _returnvalue_2))