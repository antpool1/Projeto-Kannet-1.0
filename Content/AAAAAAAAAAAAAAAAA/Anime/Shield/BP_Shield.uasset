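; BP_Shield is a shield actor set up for a throw that homes in on enemies, but the throw is unfinished.
; BeginPlay and ActivateShieldThrow are empty; the nodes for caching the player, detaching, finding nearby pawns and setting the ProjectileMovement homing target are unconnected and never run.
; ShieldReference returns the actor itself.
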(event Custom|Activate%20Shield%20Throw
  ;[0.05098 0.05098 0.05098] Shield
)

(event EventBeginPlay
  ;[0.05098 0.05098 0.05098] Shield
)

(fn ConstructionScript)

(fn ShieldReference
  (return self))